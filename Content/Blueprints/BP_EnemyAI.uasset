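; Enemy AI character that chases the first player on sight and knocks characters back with an attack.
; PawnSensing triggers an AI MoveTo toward the player, and arrival plays the attack montage if CanAttack allows.
; CanAttack stays false until the montage completes or is interrupted.
; A montage notify fires a debug-drawn forward sphere trace that launches a hit Character forward and up, without applying damage.
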(event OnSeePawn(PawnSensing)
  (params (Pawn :type Pawn%20Object%20Reference))
  (CallFunction|ChasePlayer))

(event Custom|ChasePlayer
  (bind _returnvalue (Transformation|GetActorLocation))
  (AI|AIMoveTo self "0, 0, 0" (Game|GetPlayerCharacter 0) 1e+02 false
    (:OnSuccess
      (if (Variables|Default|GetcanAttack?)
        (Animation|Montage|PlayMontage (Variables|Character|GetMesh) "/Game/Characters/Villager/Animations/Attack/A_Attack_Montage.A_Attack_Montage"
          (:then
            (Variables|Default|SetcanAttack? false))
          (:OnCompleted
            (Variables|Default|SetcanAttack? true :!label _label))
          (:OnInterrupted
            (goto _label))
          (:OnNotifyBegin
            (bind _outhit (Collision|SphereTraceByChannel _returnvalue (+ _returnvalue (* (Math|Vector|GetForwardVector (Transformation|GetActorRotation)) 1.8e+02)) 25.0 "TraceTypeQuery3" false 0 "ForDuration"))
            (if true
              (bind _ascharacter (Utilities|Casting|CastToCharacter (.HitActor (Collision|BreakHitResult _outhit))))
              (Character|LaunchCharacter _ascharacter (+ (* (Math|Vector|GetForwardVector (Transformation|GetActorRotation)) (Variables|Default|GetfrontKnockback)) (Math|Vector|MakeVector 0.0 0.0 (Variables|Default|GetupwardsKnockback))) false false))))))))

(event EventBeginPlay)

(fn ConstructionScript)